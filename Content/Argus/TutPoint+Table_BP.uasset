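; VR tutorial sequencer actor that walks the player through narrated wristband button, pointing, grabbing, teleport and object-placement lessons.
; BeginPlay hides later props, caches hand and object references, then cues a flashing, rumbling wristband.
; Overlaps on the point sphere, teleport zone and three slots advance TutorialStage and reveal props, ending with the dial once all slots fill.
; Tick uses a one-second Delay to poll for the button press and drive the countdown.
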(event OnComponentBeginOverlap(TeleportCollision)
  (params (OverlappedComponent :type Primitive%20Component%20Object%20Reference) (OtherActor :type Actor%20Object%20Reference) (OtherComp :type Primitive%20Component%20Object%20Reference) (OtherBodyIndex :type Integer) (bFromSweep :type Boolean) (SweepResult :type Hit%20Result%20Structure%20%28by%20ref%29))
  ;[1 1 1] Player enters teleportation zone
  (Utilities|Casting|CastToBP_MotionController OtherActor)
  (Audio|PlaySound2D "/Game/Argus/Audio/S_correct_beep_Cue.S_correct_beep_Cue")
  (Audio|Components|Audio|Stop (Variables|Default|GetTeleportAudio))
  (Variables|Default|SettutorialStage 8)
  ;;[1 1 1] Begin grab 2 section
  (Audio|PlaySound2D "/Game/Argus/Audio/TutD5_S2.TutD5_S2")
  (Utilities|FlowControl|Delay 2.0)
  (Rendering|SetVisibility (Variables|Default|GetTable2) true true)
  (Rendering|SetVisibility (Variables|/Script/Engine.StaticMeshActor|GetStaticMeshComponent (Variables|Default|GetTutGrab2REF)) true false)
  (Rendering|SetVisibility (Variables|Default|GetCountdown) false false)
  ;;[1 1 1] turn off teleport zone
  (Rendering|SetVisibility (Variables|Default|GetTeleportZone) true true)
  (Collision|SetCollisionEnabled (Variables|Default|GetTeleportCollision) "NoCollision"))

(event OnComponentBeginOverlap(slot3)
  (params (OverlappedComponent :type Primitive%20Component%20Object%20Reference) (OtherActor :type Actor%20Object%20Reference) (OtherComp :type Primitive%20Component%20Object%20Reference) (OtherBodyIndex :type Integer) (bFromSweep :type Boolean) (SweepResult :type Hit%20Result%20Structure%20%28by%20ref%29))
  (bind _tutgrab3ref (Variables|Default|GetTutGrab3REF))
  (bind _dialref (Variables|Default|GetDialREF))
  (bind _staticmeshcomponent (Variables|/Script/Engine.StaticMeshActor|GetStaticMeshComponent _tutgrab3ref))
  ;[1 1 1] object 3 grab in slot 3
  (if (== OtherActor (Variables|Default|GetTutGrab3REF)) ; If player is grabbing the right cube, then they've teleported successfully
    (Rendering|Material|SetVectorParameterValueonMaterials (Variables|Default|Getslot3) "Color" "0,1.000000, 0")
    (Audio|PlaySound2D "/Game/Argus/Audio/S_correct_beep_Cue.S_correct_beep_Cue")
    ;[1 1 1] Player can't grab cube again
    (Variables|/Script/Engine.PrimitiveComponent|SetbGenerateOverlapEvents _staticmeshcomponent false)
    (Collision|SetCollisionEnabled _staticmeshcomponent "NoCollision")
    (Physics|SetSimulatePhysics _staticmeshcomponent false)
    (Math|Integer|IncrementInt (Variables|Default|GetobjectPlaced)
      (:%20%20
        (if (== (Variables|Default|GetobjectPlaced) 3)
          ;[1 1 1] Dial Box instructions
          (Variables|Default|SettutorialStage 11)
          (Variables|Default|SetbeginCountdown? false)
          (Utilities|FlowControl|Delay 2.0)
          (Audio|PlaySound2D "/Game/Argus/Audio/TutD9.TutD9")
          (Utilities|FlowControl|Delay 2.0)
          (Rendering|SetVisibility (Variables|/Game/Argus/Dial1BP.Dial1BP_C|GetDefaultSceneRoot _dialref) true true) ; Turn on dial section
          (Rendering|SetVisibility (Variables|/Game/Argus/Dial1BP.Dial1BP_C|GetDoor _dialref) false false)
          (Rendering|SetVisibility (Variables|/Game/Argus/Dial1BP.Dial1BP_C|GetDial _dialref) true true)
          (Utilities|FlowControl|Delay 7.0))))))

(event OnComponentBeginOverlap(pointSphere)
  (params (OverlappedComponent :type Primitive%20Component%20Object%20Reference) (OtherActor :type Actor%20Object%20Reference) (OtherComp :type Primitive%20Component%20Object%20Reference) (OtherBodyIndex :type Integer) (bFromSweep :type Boolean) (SweepResult :type Hit%20Result%20Structure%20%28by%20ref%29))
  (bind _tutgrab1ref (Variables|Default|GetTutGrab1REF))
  (bind _pointsphere (Variables|Default|GetpointSphere))
  (bind _staticmeshcomponent (Variables|/Script/Engine.StaticMeshActor|GetStaticMeshComponent _tutgrab1ref))
  ;[1 1 1] If player selects sphere, turn it green, then play 'correct' beep and Circe, then start grab tutorial
  (Utilities|Casting|CastToBP_MotionController OtherActor) ; Check if overlapping objec is the pointer
  (if (and (Variables|Default|GetfinishPointExplain?) (Math|Boolean|Equal(Boolean) (Variables|Default|GetpointTutFinish?) false)) ; if pointer was detected, point explaination is finished, and point tutorial is NOT finished, then...
    (Audio|PlaySound2D "/Game/Argus/Audio/S_correct_beep_Cue.S_correct_beep_Cue")
    (Rendering|Material|SetVectorParameterValueonMaterials _pointsphere "DiffuseColor" "0,1.000000, 0") ; Turn point sphere green
    (bind _fadedtaa (Timeline|FadeOpacity Play) ; Fade DTAA
      (:Update
        (Rendering|Material|SetScalarParameterValueonMaterials _pointsphere "DTAA" _fadedtaa))
      (:Finished
        (Rendering|SetVisibility _pointsphere false false)
        (Utilities|FlowControl|Delay 1.0)
        (Audio|PlaySound2D "/Game/Argus/Audio/TutD4.TutD4") ; Start grabbing instruction
        (Variables|Default|SetpointTutFinish? true)
        (Utilities|FlowControl|Delay 8.0)
        (Audio|PlaySound2D "/Game/Argus/Audio/TutD4_grab.TutD4_grab")
        (Variables|Default|SettutorialStage 5)
        (Utilities|FlowControl|Delay 2.0)
        (Rendering|SetVisibility _staticmeshcomponent true false)
        (Collision|SetCollisionEnabled _staticmeshcomponent "QueryAndPhysics")))))

(event OnComponentBeginOverlap(Slot1)
  (params (OverlappedComponent :type Primitive%20Component%20Object%20Reference) (OtherActor :type Actor%20Object%20Reference) (OtherComp :type Primitive%20Component%20Object%20Reference) (OtherBodyIndex :type Integer) (bFromSweep :type Boolean) (SweepResult :type Hit%20Result%20Structure%20%28by%20ref%29))
  (bind _dialref (Variables|Default|GetDialREF))
  (bind _tutgrab2ref (Variables|Default|GetTutGrab2REF))
  (bind _staticmeshcomponent (Variables|/Script/Engine.StaticMeshActor|GetStaticMeshComponent _tutgrab2ref))
  ;[1 1 1] When slot 1 overlaps with object2 from 2nd table,
  (if (== OtherActor (Variables|Default|GetTutGrab2REF)) ; If player is grabbing the right cube, then they've teleported successfully
    (Variables|Default|SetteleportTutFinish? true)
    (Rendering|Material|SetVectorParameterValueonMaterials (Variables|Default|Getslot1) "Color" "0,1.000000, 0")
    (Audio|PlaySound2D "/Game/Argus/Audio/S_correct_beep_Cue.S_correct_beep_Cue")
    (Variables|Default|SettutorialStage 10)
    ;[1 1 1] Instruct player to fill other slots with two objects, make object 1 and 3 visible
    (Utilities|FlowControl|Delay 2.0)
    (Audio|PlaySound2D "/Game/Argus/Audio/TutD7.TutD7")
    (Audio|PlaySound2D 0) ; Play ticking noise, will increase as countdown ends
    (Rendering|SetVisibility (Variables|Default|Getpodium) true false)
    (Rendering|SetVisibility (Variables|/Script/Engine.StaticMeshActor|GetStaticMeshComponent (Variables|Default|GetTutGrab3REF)) true false)
    (Variables|Default|SetNeedGrab1? true)
    (Variables|Default|SetbeginCountdown? true)
    ;[1 1 1] Player can't grab cube again
    (Variables|/Script/Engine.PrimitiveComponent|SetbGenerateOverlapEvents _staticmeshcomponent false)
    (Collision|SetCollisionEnabled _staticmeshcomponent "NoCollision")
    (Physics|SetSimulatePhysics _staticmeshcomponent false)
    (Math|Integer|IncrementInt (Variables|Default|GetobjectPlaced)
      (:%20%20
        (if (== (Variables|Default|GetobjectPlaced) 3)
          ;[1 1 1] Dial Box instructions
          (Variables|Default|SettutorialStage 11)
          (Variables|Default|SetbeginCountdown? false)
          (Utilities|FlowControl|Delay 2.0)
          (Audio|PlaySound2D "/Game/Argus/Audio/TutD9.TutD9")
          (Utilities|FlowControl|Delay 2.0)
          (Rendering|SetVisibility (Variables|/Game/Argus/Dial1BP.Dial1BP_C|GetDefaultSceneRoot _dialref) true true) ; Turn on dial section
          (Rendering|SetVisibility (Variables|/Game/Argus/Dial1BP.Dial1BP_C|GetDoor _dialref) false false)
          (Rendering|SetVisibility (Variables|/Game/Argus/Dial1BP.Dial1BP_C|GetDial _dialref) true true)
          (Utilities|FlowControl|Delay 7.0))))))

(event OnComponentBeginOverlap(slot2)
  (params (OverlappedComponent :type Primitive%20Component%20Object%20Reference) (OtherActor :type Actor%20Object%20Reference) (OtherComp :type Primitive%20Component%20Object%20Reference) (OtherBodyIndex :type Integer) (bFromSweep :type Boolean) (SweepResult :type Hit%20Result%20Structure%20%28by%20ref%29))
  (bind _dialref (Variables|Default|GetDialREF))
  (bind _tutgrab1ref (Variables|Default|GetTutGrab1REF))
  (bind _staticmeshcomponent (Variables|/Script/Engine.StaticMeshActor|GetStaticMeshComponent _tutgrab1ref))
  ;[1 1 1] Object1 grab in slot 2
  (if (== OtherActor (Variables|Default|GetTutGrab1REF)) ; If player is grabbing the right cube, then they've teleported successfully
    (Rendering|Material|SetVectorParameterValueonMaterials (Variables|Default|GetSlot2) "Color" "0,1.000000, 0")
    (Audio|PlaySound2D "/Game/Argus/Audio/S_correct_beep_Cue.S_correct_beep_Cue")
    ;[1 1 1] Player can't grab cube again
    (Variables|/Script/Engine.PrimitiveComponent|SetbGenerateOverlapEvents _staticmeshcomponent false)
    (Collision|SetCollisionEnabled _staticmeshcomponent "NoCollision")
    (Physics|SetSimulatePhysics _staticmeshcomponent false)
    (Math|Integer|IncrementInt (Variables|Default|GetobjectPlaced)
      (:%20%20
        (if (== (Variables|Default|GetobjectPlaced) 3)
          ;[1 1 1] Dial Box instructions
          (Variables|Default|SettutorialStage 11)
          (Variables|Default|SetbeginCountdown? false)
          (Utilities|FlowControl|Delay 2.0)
          (Audio|PlaySound2D "/Game/Argus/Audio/TutD9.TutD9")
          (Utilities|FlowControl|Delay 2.0)
          (Rendering|SetVisibility (Variables|/Game/Argus/Dial1BP.Dial1BP_C|GetDefaultSceneRoot _dialref) true true) ; Turn on dial section
          (Rendering|SetVisibility (Variables|/Game/Argus/Dial1BP.Dial1BP_C|GetDoor _dialref) false false)
          (Rendering|SetVisibility (Variables|/Game/Argus/Dial1BP.Dial1BP_C|GetDial _dialref) true true)
          (Utilities|FlowControl|Delay 7.0))))))

(event EventBeginPlay
  (bind _righthandref (Variables|Default|GetRightHandREF))
  (bind _wristband (Variables|/Game/VirtualRealityBP/Blueprints/BP_MotionController.BP_MotionController_C|Getwristband _righthandref))
  (CameraFades|StartCameraFade :self (Game|GetPlayerCameraManager 0) :FromAlpha 1.0 :Duration 0.8)
  ;[1 1 1] Call being play settings function
  (CallFunction|BeginPlaySettings)
  (Utilities|FlowControl|Delay 2.0)
  ;[1 1 1] circe intro
  (Audio|PlaySound2D "/Game/Argus/Audio/TutD1_S1.TutD1_S1") ; Circe welcomes player instrcts them to press A
  ;[1 1 1] Right hand glow set up
  (Utilities|FlowControl|Delay 12.0)
  (Rendering|Material|SetVectorParameterValueonMaterials _wristband "BaseColor" "1.000000,0.000000,0.000000") ; change base color to red, flashing 1
  (Rendering|Material|SetScalarParameterValueonMaterials _wristband "Frequency" 1.0)
  (Default|RumbleController _righthandref 0.3 true)
  ;[1 1 1] Tell player to press A button
  (Variables|Default|SettutorialStage 1)
  (Utilities|FlowControl|Delay 1.0)
  (Variables|Default|SetCirceTutD1S1_Finished? true))

(event Collision|EventActorBeginOverlap
  (params (OtherActor :type Actor%20Object%20Reference)))

(event EventTick
  (params (DeltaSeconds :type Float%20%28single-precision%29))
  (bind _pointsphere (Variables|Default|GetpointSphere))
  (bind _righthandref (Variables|Default|GetRightHandREF))
  (bind _countdown (Variables|Default|GetCountdown))
  (bind _wristband (Variables|/Game/VirtualRealityBP/Blueprints/BP_MotionController.BP_MotionController_C|Getwristband _righthandref))
  ;[1 1 1] Updated current time variable until not needed
  (Utilities|FlowControl|Delay 1.0)
  (Utilities|FlowControl|Sequence
    (:then_0
      ;[1 1 1] If right hand presses A button --> it will turn green and fade out using DTAA --> then set BeginIntro to true
      (if (Math|Boolean|ANDBoolean (Variables|/Game/VirtualRealityBP/Blueprints/BP_MotionController.BP_MotionController_C|GetPlayerHUDOn? (Variables|Default|GetRightHandREF)) (Math|Boolean|Equal(Boolean) (Variables|Default|GetBeginIntro?) false) (Variables|Default|GetCirceTutD1S1_Finished?)) ; Is player activiating right hand HUD menu?
        (Variables|Default|SettutorialStage 2)
        (Audio|PlaySound2D "/Game/Argus/Audio/S_correct_beep_Cue.S_correct_beep_Cue" 0.1)
        (Default|RumbleController _righthandref 0.0 false) ; Turn off vibration
        (Rendering|Material|SetVectorParameterValueonMaterials _wristband "BaseColor" "0.000000,1.000000, 0") ; change button color to green, flashing 0
        (Rendering|Material|SetScalarParameterValueonMaterials _wristband "Frequency" 0.0)
        (Variables|Default|SetBeginIntro? true)
        (bind _colorfade (Timeline|FadeOut Play) ; Fade base color from green to white
          (:Update
            (Rendering|Material|SetVectorParameterValueonMaterials _wristband "BaseColor" (Math|Conversions|ToVector(LinearColor) _colorfade))
            (Utilities|FlowControl|Delay 2.0)
            (Audio|PlaySound2D "/Game/Argus/Audio/TutD1_S2.TutD1_S2")
            (Utilities|FlowControl|Delay 11.0)
            ;[1 1 1] If button pushed, start tutorial intro
            (if (Variables|Default|GetBeginIntro?)
              ;[1 1 1] Circe instructs player on blue circle and pointer
              (Audio|PlaySound2D "/Game/Argus/Audio/TutD1_S3.TutD1_S3")
              (Variables|Default|SettutorialStage 3)
              (Utilities|FlowControl|Delay 4.0)
              (Audio|PlaySound2D "/Game/Argus/Audio/TutD2.TutD2") ; Blue Circle demo
              (Utilities|FlowControl|Delay 9.0)
              (Variables|Default|SettutorialStage 4)
              (Audio|PlaySound2D "/Game/Argus/Audio/TutD3.TutD3") ; Selection demo
              (Utilities|FlowControl|Delay 2.0)
              (Utilities|FlowControl|Delay 5.0)
              (Variables|Default|SetfinishPointExplain? true)
              (Variables|/Script/Engine.PrimitiveComponent|SetbGenerateOverlapEvents _pointsphere true)
              (Rendering|SetVisibility _pointsphere true false))))))
    (:then_1
      (if (Variables|Default|GetbeginCountdown?)
        (Rendering|SetVisibility _countdown true false)
        (CallFunction|HandleCountdown)
        (else
          (Rendering|SetVisibility _countdown false false))))))

(fn ConstructionScript)

(fn BeginPlaySettings
  (Utilities|FlowControl|Sequence
    (:then_0
      ;[1 1 1] Boolean variables
      (Variables|Default|SetfinishPointExplain? false)
      (Variables|Default|SetpointTutFinish? false)
      (Variables|Default|SetbeginCountdown? false)
      (Variables|Default|SetCirceTutD1S1_Finished? false)
      (Variables|Default|SettutorialStage 0)
      (Variables|Default|SetTimeMin 1)
      (Variables|Default|SetTimeSec 30)
      (Variables|Default|SetcountdownOver false)
      (Variables|Default|SetcountdownOver false))
    (:then_1
      ;[1 1 1] Get Tutorial Grab1 and set invisible & collision disabled
      (bind _outactors (Actor|GetAllActorsOfClass "/Game/Argus/TutGrab1_BP.TutGrab1_BP_C"))
      (Utilities|IsValid (Utilities|Array|Get(acopy) _outactors)
        (:Is%20Valid
          (bind _output_get (Variables|Default|SetTutGrab1REF (Utilities|Array|Get(acopy) _outactors)))
          (Rendering|SetVisibility (Variables|/Script/Engine.StaticMeshActor|GetStaticMeshComponent _output_get) false false) ; Make the grab1 object invisible so that player can focus on pointing
          (Collision|SetCollisionEnabled (Variables|/Script/Engine.StaticMeshActor|GetStaticMeshComponent _output_get) "NoCollision")
          (bind _outactors_2 (Actor|GetAllActorsOfClass "/Game/Argus/TutGrab2_BP.TutGrab2_BP_C")) ; Check if slot 1 collided with grab2
          (Variables|Default|SetTutGrab2REF (Utilities|Array|Get(acopy) _outactors_2)))))
    (:then_2
      ;[1 1 1] Set podium invisible & objectPlaced to 0
      (Rendering|SetVisibility (Variables|Default|Getpodium) false false)
      (Variables|Default|SetobjectPlaced 0))
    (:then_3
      ;[1 1 1] Get Tutorial Grab3 and set invisible
      (bind _outactors_3 (Actor|GetAllActorsOfClass "/Game/Argus/TutGrab3_BP.TutGrab3_BP_C"))
      (Utilities|IsValid (Utilities|Array|Get(acopy) _outactors_3)
        (:Is%20Valid
          (bind _output_get_2 (Variables|Default|SetTutGrab3REF (Utilities|Array|Get(acopy) _outactors_3)))
          (Rendering|SetVisibility (Variables|/Script/Engine.StaticMeshActor|GetStaticMeshComponent _output_get_2) false false))))
    (:then_4
      ;[1 1 1] Get Dial components and set invisible
      (bind _outactors_4 (Actor|GetAllActorsOfClass "/Game/Argus/Dial1BP.Dial1BP_C"))
      (Utilities|IsValid (Utilities|Array|Get(acopy) _outactors_4)
        (:Is%20Valid
          (bind _output_get_3 (Variables|Default|SetDialREF (Utilities|Array|Get(acopy) _outactors_4)))
          (Rendering|SetVisibility (Variables|/Game/Argus/Dial1BP.Dial1BP_C|GetDefaultSceneRoot _output_get_3) false true)
          (Rendering|SetVisibility (Variables|/Game/Argus/Dial1BP.Dial1BP_C|GetDial _output_get_3) false true))))
    (:then_5
      (Rendering|SetVisibility (Variables|Default|GetpointSphere) false false)
      (Rendering|SetVisibility (Variables|Default|GetTable2) false true)
      (Rendering|SetVisibility (Variables|/Script/Engine.StaticMeshActor|GetStaticMeshComponent (Variables|Default|GetTutGrab2REF)) false false))
    (:then_6
      (bind _outactors_5 (Actor|GetAllActorsOfClass "/Game/VirtualRealityBP/Blueprints/MotionControllerPawn.MotionControllerPawn_C"))
      (Variables|Default|SetLeftHandREF (Variables|/Game/VirtualRealityBP/Blueprints/MotionControllerPawn.MotionControllerPawn_C|GetLeftController (Utilities|Array|Get(acopy) _outactors_5)))
      (Variables|Default|SetRightHandREF (Variables|/Game/VirtualRealityBP/Blueprints/MotionControllerPawn.MotionControllerPawn_C|GetRightController (Utilities|Array|Get(acopy) _outactors_5))))
    (:then_7
      (bind _outactors_6 (Actor|GetAllActorsOfClass "/Game/Argus/BP_PlayerHUD.BP_PlayerHUD_C"))
      (Variables|Default|SetPlayerHUDREF (Utilities|Array|Get(acopy) _outactors_6)))
    (:then_8
      (Rendering|SetVisibility (Variables|Default|GetTeleportZone) false true)
      (Audio|Components|Audio|Stop (Variables|Default|GetTeleportAudio)))
    (:then_9
      (Rendering|Material|CreateDynamicMaterialInstance (Variables|/Game/VirtualRealityBP/Blueprints/BP_MotionController.BP_MotionController_C|Getwristband (Variables|Default|GetRightHandREF)) 0 "/Game/Argus/Materials/Wristband_MAT.Wristband_MAT" :!class /Script/Engine.PrimitiveComponent)
      (Rendering|Material|SetVectorParameterValueonMaterials (Variables|/Game/VirtualRealityBP/Blueprints/BP_MotionController.BP_MotionController_C|Getwristband (Variables|Default|GetRightHandREF)) "BaseColor" "1.000000,1.000000,1.000000") ; change button color to white, flashing 0
      (Rendering|Material|SetScalarParameterValueonMaterials (Variables|/Game/VirtualRealityBP/Blueprints/BP_MotionController.BP_MotionController_C|Getwristband (Variables|Default|GetRightHandREF)) "Frequency" 0.0))))

(fn HandleCountdown
  (bind _output_get (Variables|Default|SetTimeSec (- (Variables|Default|GetTimeSec) 1)))
  (if (== _output_get 0)
    (Variables|Default|SetTimeMin (- (Variables|Default|GetTimeMin) 1))
    (Variables|Default|SetTimeSec 59)
    (if (== (+ (Variables|Default|GetTimeSec) (Variables|Default|GetTimeMin)) 0)
      (Variables|Default|SetcountdownOver true)
      (else
        (Variables|Default|SetcountdownOver false)))))