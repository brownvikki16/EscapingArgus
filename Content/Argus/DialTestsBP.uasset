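; Test Blueprint for VR dials that turn with the roll of the player's hand.
; Dial 3 is grabbed through Pickup and Drop events, while Dial 2 engages by overlapping the first motion controller's hand mesh.
; Tick calls RotateDialOnGrab, setting each active dial's world roll from RightHandREF with inverted, amplified rotation and fixed pitch and yaw.
; Only Pickup sets RightHandREF, so Dial 2 also depends on it.
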(event OnComponentBeginOverlap(Dial2)
  (params (OverlappedComponent :type Primitive%20Component%20Object%20Reference) (OtherActor :type Actor%20Object%20Reference) (OtherComp :type Primitive%20Component%20Object%20Reference) (OtherBodyIndex :type Integer) (bFromSweep :type Boolean) (SweepResult :type Hit%20Result%20Structure%20%28by%20ref%29))
  (bind _outactors (Actor|GetAllActorsOfClass "/Game/VirtualRealityBP/Blueprints/BP_MotionController.BP_MotionController_C"))
  (if (== OtherComp (Variables|/Game/VirtualRealityBP/Blueprints/BP_MotionController.BP_MotionController_C|GetHandMesh (Utilities|Array|Get(acopy) _outactors)))
    (Variables|Default|SetDial2Grabbed? true)))

(event OnComponentEndOverlap(Dial2)
  (params (OverlappedComponent :type Primitive%20Component%20Object%20Reference) (OtherActor :type Actor%20Object%20Reference) (OtherComp :type Primitive%20Component%20Object%20Reference) (OtherBodyIndex :type Integer))
  (Variables|Default|SetDial2Grabbed? false))

(event EventBeginPlay
  (Variables|Default|SetDial3Grabbed? false)
  (Variables|Default|SetDial2Grabbed? false))

(event Collision|EventActorBeginOverlap
  (params (OtherActor :type Actor%20Object%20Reference)))

(event EventTick
  (params (DeltaSeconds :type Float%20%28single-precision%29))
  (Utilities|FlowControl|Sequence
    (:then_0
      (if (Variables|Default|GetDial3Grabbed?)
        (CallFunction|RotateDialonGrab)))
    (:then_1
      (if (Variables|Default|GetDial2Grabbed?)
        (CallFunction|RotateDialonGrab)))))

(event EventPickup
  (params (AttachTo :type Scene%20Component%20Object%20Reference))
  ;[1 1 1] Dial 3 pickup and let go system
  (Variables|Default|SetRightHandREF AttachTo)
  (Variables|Default|SetDial3Grabbed? true))

(event EventDrop
  ;[1 1 1] Dial 3 pickup and let go system
  (Variables|Default|SetDial3Grabbed? false))

(fn ConstructionScript)

(fn RotateDialonGrab
  (Utilities|FlowControl|Sequence
    (:then_0
      (if (Variables|Default|GetDial3Grabbed?)
        (Transformation|SetWorldRotation (Variables|Default|GetDial3) (Math|Rotator|MakeRotator (* (.roll (Transformation|GetWorldRotation (Variables|Default|GetRightHandREF))) -2.0) 0.0 9e+01) false false)))
    (:then_1
      (if (Variables|Default|GetDial2Grabbed?)
        (Transformation|SetWorldRotation (Variables|Default|GetDial2) (Math|Rotator|MakeRotator (* (.roll (Transformation|GetWorldRotation (Variables|Default|GetRightHandREF))) -2.0) 0.0 9e+01) false false)))))