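; Grabbable VR tutorial object that completes the grabbing lesson and introduces the teleport lesson.
; On BeginPlay it caches and hides the second table from TutPointTable_BP and the mesh from TutGrab2_BP.
; Pickup, called by BP_MotionController, attaches it with physics off, and Drop reverses this.
; The first pickup turns it green, plays a beep and teleport instructions, then reveals the hidden table and object after timed delays.
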(event EventBeginPlay
  ;[1 1 1] Set variables at start adn make Grab tut 2 features and 2nd table invisible
  (Variables|Default|SetObjectGrabbed? false)
  (Variables|Default|SetTeleport&Grabbed? false)
  (bind _outactors (Actor|GetAllActorsOfClass "/Game/Argus/TutPoint+Table_BP.TutPoint+Table_BP_C"))
  (Utilities|IsValid (Utilities|Array|Get(acopy) _outactors)
    (:Is%20Valid
      (Variables|Default|Settable2REF (Variables|/Game/Argus/TutPoint+Table_BP.TutPoint+Table_BP_C|GetTable2 (Utilities|Array|Get(acopy) _outactors)))
      (Rendering|SetVisibility (Variables|/Game/Argus/TutPoint+Table_BP.TutPoint+Table_BP_C|GetTable2 (Utilities|Array|Get(acopy) _outactors)) false true) ; Make the table2 object invisible before teleporting stage
      (bind _outactors_2 (Actor|GetAllActorsOfClass "/Game/Argus/TutGrab2_BP.TutGrab2_BP_C"))
      (Utilities|IsValid (Utilities|Array|Get(acopy) _outactors_2)
        (:Is%20Valid
          (bind _output_get (Variables|Default|Setgrab2REF (Variables|/Script/Engine.StaticMeshActor|GetStaticMeshComponent (Utilities|Array|Get(acopy) _outactors_2))))
          (Rendering|SetVisibility _output_get false false))))))

(event Collision|EventActorBeginOverlap
  (params (OtherActor :type Actor%20Object%20Reference)))

(event EventTick
  (params (DeltaSeconds :type Float%20%28single-precision%29)))

(event EventPickup
  (params (AttachTo :type Scene%20Component%20Object%20Reference))
  (Physics|SetSimulatePhysics (Variables|Debug|GetStaticMeshComponent) false)
  (Transformation|AttachComponentToComponent (VehicleSound|GetRootComponent) AttachTo "eve" "KeepWorld" "KeepWorld" "KeepWorld" false)
  (if (not (Variables|Default|GetObjectGrabbed?)) ; has the grabbing tutorial been completed?
    ;[1 1 1] completing grabbing tutorial
    (Rendering|Material|SetVectorParameterValueonMaterials (Variables|Debug|GetStaticMeshComponent) "DiffuseColor" "0,1.000000, 0")
    (Audio|PlaySound2D "/Game/Argus/Audio/S_correct_beep_Cue.S_correct_beep_Cue")
    (Utilities|FlowControl|Delay 2.0)
    ;[1 1 1] begin teleport instructions
    (Audio|PlaySound2D "/Game/Argus/Audio/TutD5.TutD5")
    (Variables|Default|SetObjectGrabbed? true)
    (Utilities|FlowControl|Delay 28.5)
    (Rendering|SetVisibility (Variables|Default|Gettable2REF) true true)
    (Rendering|SetVisibility (Variables|Default|Getgrab2REF) true false)
    (Utilities|FlowControl|Delay 1.0)))

(event EventDrop
  (Physics|SetSimulatePhysics (Variables|Debug|GetStaticMeshComponent) true)
  (Transformation|DetachFromActor "KeepWorld" "KeepWorld" "KeepWorld"))

(fn ConstructionScript)