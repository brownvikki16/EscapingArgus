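; Tutorial VR dial that the player grabs and turns to find a target range, cued by controller rumble and color.
; While grabbed, hand height slides the Holder vertically and sets the dial's pitch.
; DialDetect overlaps with Range1 and Range12 rumble the right controller lightly; Range2 rumbles fully and fades the dial toward green.
; Leaving Range2 after full green completes the tutorial, playing audio and showing a placeholder Door; leaving earlier reverses the fade.
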(event OnComponentEndOverlap(Range1)
  (params (OverlappedComponent :type Primitive%20Component%20Object%20Reference) (OtherActor :type Actor%20Object%20Reference) (OtherComp :type Primitive%20Component%20Object%20Reference) (OtherBodyIndex :type Integer))
  ;[1 1 1] Vibrate left hand controller for player contact with range 1
  (Default|RumbleController (Variables|/Game/VirtualRealityBP/Blueprints/MotionControllerPawn.MotionControllerPawn_C|GetRightController (Variables|Default|GetControllerPawnREF)) 0.0 false))

(event OnComponentEndOverlap(Range2)
  (params (OverlappedComponent :type Primitive%20Component%20Object%20Reference) (OtherActor :type Actor%20Object%20Reference) (OtherComp :type Primitive%20Component%20Object%20Reference) (OtherBodyIndex :type Integer))
  ;[1 1 1] Logic for player contact with range 2
  (Default|RumbleController (Variables|/Game/VirtualRealityBP/Blueprints/MotionControllerPawn.MotionControllerPawn_C|GetRightController (Variables|Default|GetControllerPawnREF)) 0.0 false) ; stop the rumble loop
  (if (Variables|Default|GetRange2Detected?) ; check if player held on range 2 long enough
    (Variables|Default|SetDialTutDone? true)
    (Variables|/Script/Engine.PrimitiveComponent|SetbGenerateOverlapEvents (Variables|Default|GetDialDetect) false) ; Turn off dial detect to stop vibrations
    (Utilities|FlowControl|Delay 1.0)
    (Audio|PlaySound2D "/Game/Argus/Audio/TutD10.TutD10")
    (Utilities|FlowControl|Delay 3.0)
    (Rendering|SetVisibility (Variables|Default|GetDoor) true false) ; place holder for door sliding up
    (elif (not (Variables|Default|GetDialTutDone?))
      (bind _fadetogreen (Timeline|ColorChange Reverse)
        (:Update
          (Rendering|Material|SetVectorParameterValueonMaterials (Variables|Default|GetDial) "Color" (Math|Conversions|ToVector(LinearColor) _fadetogreen))
          (Variables|Default|SetRange2Detected? (Math|Vector|Equal(Vector) (Math|Conversions|ToVector(LinearColor) _fadetogreen) (Variables|Default|GetGreenColor) 0.0001)))))))

(event OnComponentBeginOverlap(Range1-2)
  (params (OverlappedComponent :type Primitive%20Component%20Object%20Reference) (OtherActor :type Actor%20Object%20Reference) (OtherComp :type Primitive%20Component%20Object%20Reference) (OtherBodyIndex :type Integer) (bFromSweep :type Boolean) (SweepResult :type Hit%20Result%20Structure%20%28by%20ref%29))
  ;[1 1 1] Vibrate left hand controller for player contact with range 1-2
  (if (== OtherComp (Variables|Default|GetDialDetect))
    (Default|RumbleController (Variables|/Game/VirtualRealityBP/Blueprints/MotionControllerPawn.MotionControllerPawn_C|GetRightController (Variables|Default|GetControllerPawnREF)) 0.3 true)))

(event OnComponentEndOverlap(Range1-2)
  (params (OverlappedComponent :type Primitive%20Component%20Object%20Reference) (OtherActor :type Actor%20Object%20Reference) (OtherComp :type Primitive%20Component%20Object%20Reference) (OtherBodyIndex :type Integer))
  ;[1 1 1] Vibrate left hand controller for player contact with range 1-2
  (Default|RumbleController (Variables|/Game/VirtualRealityBP/Blueprints/MotionControllerPawn.MotionControllerPawn_C|GetRightController (Variables|Default|GetControllerPawnREF)) 0.0 false))

(event OnComponentBeginOverlap(Range1)
  (params (OverlappedComponent :type Primitive%20Component%20Object%20Reference) (OtherActor :type Actor%20Object%20Reference) (OtherComp :type Primitive%20Component%20Object%20Reference) (OtherBodyIndex :type Integer) (bFromSweep :type Boolean) (SweepResult :type Hit%20Result%20Structure%20%28by%20ref%29))
  ;[1 1 1] Vibrate left hand controller for player contact with range 1
  (if (== OtherComp (Variables|Default|GetDialDetect))
    (Default|RumbleController (Variables|/Game/VirtualRealityBP/Blueprints/MotionControllerPawn.MotionControllerPawn_C|GetRightController (Variables|Default|GetControllerPawnREF)) 0.3 true)))

(event OnComponentBeginOverlap(Range2)
  (params (OverlappedComponent :type Primitive%20Component%20Object%20Reference) (OtherActor :type Actor%20Object%20Reference) (OtherComp :type Primitive%20Component%20Object%20Reference) (OtherBodyIndex :type Integer) (bFromSweep :type Boolean) (SweepResult :type Hit%20Result%20Structure%20%28by%20ref%29))
  ;[1 1 1] Logic for player contact with range 2
  (if (and (== OtherComp (Variables|Default|GetDialDetect)) (Math|Boolean|Equal(Boolean) (Variables|Default|GetDialTutDone?) false)) ; check that dial detect is overlap and dial tut is not over
    (Default|RumbleController (Variables|/Game/VirtualRealityBP/Blueprints/MotionControllerPawn.MotionControllerPawn_C|GetRightController (Variables|Default|GetControllerPawnREF)) 1.0 true) ; loop the rumble
    (bind _fadetogreen (Timeline|ColorChange Play)
      (:Update
        (Rendering|Material|SetVectorParameterValueonMaterials (Variables|Default|GetDial) "Color" (Math|Conversions|ToVector(LinearColor) _fadetogreen))
        (Variables|Default|SetRange2Detected? (Math|Vector|Equal(Vector) (Math|Conversions|ToVector(LinearColor) _fadetogreen) (Variables|Default|GetGreenColor) 0.0001))))))

(event EventBeginPlay
  (Variables|Default|SetDialGrabbed? false)
  (bind _outactors (Actor|GetAllActorsOfClass "/Game/VirtualRealityBP/Blueprints/MotionControllerPawn.MotionControllerPawn_C"))
  (Variables|Default|SetControllerPawnREF (Utilities|Array|Get(acopy) _outactors))
  (Variables|Default|SetRange2Detected? false)
  (Rendering|Material|CreateDynamicMaterialInstance (Variables|Default|GetDial) 0 "/Game/StarterContent/Materials/M_Basic_Wall.M_Basic_Wall" :!class /Script/Engine.PrimitiveComponent)
  (Variables|Default|SetDialTutDone? false)
  (Variables|Default|SetHolderInitialPosition (Transformation|GetWorldLocation (Variables|Default|GetHolder))))

(event Collision|EventActorBeginOverlap
  (params (OtherActor :type Actor%20Object%20Reference)))

(event EventTick
  (params (DeltaSeconds :type Float%20%28single-precision%29))
  (if (Variables|Default|GetDialGrabbed?)
    (CallFunction|RotateDialonGrab)))

(event EventPickup
  (params (AttachTo :type Scene%20Component%20Object%20Reference))
  ;[1 1 1] Dial pickup and let go system
  (Variables|Default|SetRightHandREF AttachTo)
  (Variables|Default|SetDialGrabbed? true))

(event EventDrop
  ;[1 1 1] Dial pickup and let go system
  (Variables|Default|SetDialGrabbed? false))

(fn ConstructionScript)

(fn RotateDialonGrab
  (bind _righthandref (Variables|Default|GetRightHandREF))
  (bind _holderinitialposition (Variables|Default|GetHolderInitialPosition))
  (bind _returnvalue (Transformation|GetWorldLocation _righthandref))
  (Transformation|SetWorldLocation (Variables|Default|GetHolder) (Math|Vector|MakeVector (.x _holderinitialposition) (.y _holderinitialposition) (.z _returnvalue)) false false)
  (Transformation|SetWorldRotation (Variables|Default|GetDial) (Math|Rotator|MakeRotator 0.0 (* (.z _returnvalue) 5.0) 0.0) false false))