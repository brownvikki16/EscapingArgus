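; Round 1 trigger object that can be picked up with a motion controller and records that it has been found.
; Pickup disables physics, attaches the actor to the grabbing component, tints the mesh green through a dynamic material instance, and sets Trigger1Found.
; Drop re-enables physics and detaches it, leaving the color and flag unchanged; only BeginPlay clears the flag.
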(event EventBeginPlay
  (Variables|Default|SetTrigger1Found? false))

(event Collision|EventActorBeginOverlap
  (params (OtherActor :type Actor%20Object%20Reference)))

(event EventTick
  (params (DeltaSeconds :type Float%20%28single-precision%29)))

(event EventPickup
  (params (AttachTo :type Scene%20Component%20Object%20Reference))
  (Utilities|FlowControl|Sequence
    (:then_0
      (Physics|SetSimulatePhysics (Variables|Debug|GetStaticMeshComponent) false)
      (Transformation|AttachComponentToComponent (VehicleSound|GetRootComponent) AttachTo "eve" "KeepWorld" "KeepWorld" "KeepWorld" false))
    (:then_1
      ;[1 1 1] Set round 1 trigger color to green
      (bind _returnvalue (Rendering|Material|CreateDynamicMaterialInstance (Variables|Debug|GetStaticMeshComponent) 0 "/Game/Argus/WallLight_MAT.WallLight_MAT" :!class /Script/Engine.PrimitiveComponent))
      (Rendering|Material|SetVectorParameterValue _returnvalue "DefaultColor" (Math|Conversions|ToLinearColor(Vector) "0.000000,1.000000,0.000000") :!class /Script/Engine.MaterialInstanceDynamic))
    (:then_2
      ;[1 1 1] Set trigger 1 has been found to true
      (Variables|Default|SetTrigger1Found? true))))

(event EventDrop
  (Physics|SetSimulatePhysics (Variables|Debug|GetStaticMeshComponent) true)
  (Transformation|DetachFromActor "KeepWorld" "KeepWorld" "KeepWorld"))

(fn ConstructionScript)