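; TutGrab2_BP is the second grabbable object in a VR grab tutorial, picked up by a motion controller and meant for table slot 1.
; Pickup turns off physics and attaches the actor to the given component, and Drop detaches it and re-enables physics.
; The first pickup also turns the mesh green, plays a beep and a voice line, and advances the TutPointTable_BP found at BeginPlay to tutorial stage 9.
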(event EventBeginPlay
  (Variables|Default|SetObjectGrabbed? false)
  (bind _outactors (Actor|GetAllActorsOfClass "/Game/Argus/TutPoint+Table_BP.TutPoint+Table_BP_C"))
  (Variables|Default|SetMainTutREF (Utilities|Array|Get(acopy) _outactors)))

(event Collision|EventActorBeginOverlap
  (params (OtherActor :type Actor%20Object%20Reference)))

(event EventTick
  (params (DeltaSeconds :type Float%20%28single-precision%29)))

(event EventPickup
  (params (AttachTo :type Scene%20Component%20Object%20Reference))
  (Physics|SetSimulatePhysics (Variables|Debug|GetStaticMeshComponent) false)
  (Transformation|AttachComponentToComponent (VehicleSound|GetRootComponent) AttachTo "eve" "KeepWorld" "KeepWorld" "KeepWorld" false)
  (if (not (Variables|Default|GetObjectGrabbed?)) ; has the grabbing tutorial been completed?
    ;[1 1 1] player grabs object 2 to be placed in table slot 1
    (Rendering|Material|SetVectorParameterValueonMaterials (Variables|Debug|GetStaticMeshComponent) "DiffuseColor" "0,1.000000, 0")
    (Audio|PlaySound2D "/Game/Argus/Audio/S_correct_beep_Cue.S_correct_beep_Cue")
    (Variables|Default|SetObjectGrabbed? true)
    (Variables|/Game/Argus/TutPoint+Table_BP.TutPoint+Table_BP_C|SettutorialStage (Variables|Default|GetMainTutREF) 9)
    (Audio|PlaySound2D "/Game/Argus/Audio/TutD6.TutD6") ; play this after player has picked up grab2
    (Utilities|FlowControl|Delay 5.0)))

(event EventDrop
  (Physics|SetSimulatePhysics (Variables|Debug|GetStaticMeshComponent) true)
  (Transformation|DetachFromActor "KeepWorld" "KeepWorld" "KeepWorld"))

(fn ConstructionScript)