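; Player HUD for a VR tutorial that shows the instruction panel matching the current tutorial stage, from the welcome through pointing, grabbing, teleporting, placement and dial use.
; BeginPlay caches the tutorial table and motion controller pawn.
; Tick polls TutorialStage and toggles component visibility, swapping help display materials for pointer and teleport steps.
; After the initial hidden and Press A stages, panels show only while the right controller's PlayerHUDOn flag is set.
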(event EventBeginPlay
  (bind _outactors (Actor|GetAllActorsOfClass "/Game/Argus/TutPoint+Table_BP.TutPoint+Table_BP_C"))
  (Variables|Default|SetTutMainREF (Utilities|Array|Get(acopy) _outactors))
  (bind _outactors_2 (Actor|GetAllActorsOfClass "/Game/VirtualRealityBP/Blueprints/MotionControllerPawn.MotionControllerPawn_C"))
  (Variables|Default|SetPawnREF (Utilities|Array|Get(acopy) _outactors_2)))

(event Collision|EventActorBeginOverlap
  (params (OtherActor :type Actor%20Object%20Reference)))

(event EventTick
  (params (DeltaSeconds :type Float%20%28single-precision%29))
  (bind _helpdisplay (Variables|Default|GethelpDisplay))
  (bind _helpdisplay_2 (Variables|Default|GethelpDisplay))
  (switch int (Variables|/Game/Argus/TutPoint+Table_BP.TutPoint+Table_BP_C|GettutorialStage (Variables|Default|GetTutMainREF))
    (:Default
      (if (Variables|/Game/VirtualRealityBP/Blueprints/BP_MotionController.BP_MotionController_C|GetPlayerHUDOn? (Variables|/Game/VirtualRealityBP/Blueprints/MotionControllerPawn.MotionControllerPawn_C|GetRightController (Variables|Default|GetPawnREF)))
        (switch int (Variables|/Game/Argus/TutPoint+Table_BP.TutPoint+Table_BP_C|GettutorialStage (Variables|Default|GetTutMainREF))
          (:2
            ;[1 1 1] Welcome menu after player presses A
            (Rendering|SetVisibility (Variables|Default|GetPressA) false false)
            (Rendering|SetVisibility (Variables|Default|GethelpDisplay) false false)
            (Rendering|SetVisibility (Variables|Default|GetBG) true false)
            (Rendering|SetVisibility (Variables|Default|GetWelcome) true false))
          (:3
            ;[1 1 1] Give player main objective
            (Rendering|SetVisibility (Variables|Default|GetWelcome) false false)
            (Rendering|SetVisibility (Variables|Default|GetBG) true false)
            (Rendering|SetVisibility (Variables|Default|GetMainObj) true false))
          (:4
            ;[1 1 1] Pointer Instructions
            (Rendering|SetVisibility (Variables|Default|GetBG) true false)
            (Rendering|SetVisibility (Variables|Default|GetMainObj) false false)
            (Rendering|SetVisibility (Variables|Default|GetpointTut) true false)
            (Rendering|Material|SetMaterial _helpdisplay 0 "/Game/Argus/Materials/HelpDisplayPointer_MAT.HelpDisplayPointer_MAT")
            (Rendering|SetVisibility _helpdisplay true false))
          (:5
            ;[1 1 1] Grabbing Instructions
            (Rendering|SetVisibility (Variables|Default|GetBG) true false)
            (Rendering|SetVisibility (Variables|Default|GetpointTut) false false)
            (Rendering|SetVisibility (Variables|Default|Getgrab1Tut) true false)
            (Rendering|SetVisibility (Variables|Default|GethelpDisplay) false false))
          (:6
            ;[1 1 1] Teleporting Instructions
            (Rendering|SetVisibility (Variables|Default|GetBG) true false :!label _label)
            (Rendering|SetVisibility (Variables|Default|Getgrab1Tut) false false)
            (Rendering|SetVisibility (Variables|Default|GetteleportPt1) true true)
            (Rendering|Material|SetMaterial _helpdisplay_2 0 "/Game/Argus/Materials/HelpDisplayTeleport_MAT.HelpDisplayTeleport_MAT")
            (Rendering|SetVisibility _helpdisplay_2 true false)
            (if (== (Variables|/Game/Argus/TutPoint+Table_BP.TutPoint+Table_BP_C|GettutorialStage (Variables|Default|GetTutMainREF)) 7)
              ;[1 1 1] Teleport Instructions part 2
              (Rendering|SetVisibility (Variables|Default|GetteleportPt2) true true)))
          (:7
            (goto _label))
          (:8
            ;[1 1 1] Grab 2 instructions
            (Rendering|SetVisibility (Variables|Default|GetBG) true false)
            (Rendering|SetVisibility (Variables|Default|GetteleportPt1) false true)
            (Rendering|SetVisibility (Variables|Default|GetteleportPt2) false true)
            (Rendering|SetVisibility (Variables|Default|GethelpDisplay) false false)
            (Rendering|SetVisibility (Variables|Default|Getgrab2Tut) true false))
          (:9
            ;[1 1 1] Place cone in section 1 instructions
            (Rendering|SetVisibility (Variables|Default|GetBG) true false)
            (Rendering|SetVisibility (Variables|Default|Getgrab2Tut) false false)
            (Rendering|SetVisibility (Variables|Default|Getsection1Tut) true false))
          (:10
            ;[1 1 1] Placement tut for other sections
            (Rendering|SetVisibility (Variables|Default|GetBG) true false)
            (Rendering|SetVisibility (Variables|Default|Getsection1Tut) false false)
            (Rendering|SetVisibility (Variables|Default|GetotherSectionsTut) true false))
          (:11
            ;[1 1 1] Dial Instructions
            (Rendering|SetVisibility (Variables|Default|GetBG) true false)
            (Rendering|SetVisibility (Variables|Default|GetotherSectionsTut) false false)
            (Rendering|SetVisibility (Variables|Default|GetDialTut) true true)))
        (else
          ;[1 1 1] when A released, turn all off
          (Rendering|SetVisibility (Variables|Default|GetBG) false true)
          (Rendering|SetVisibility (Variables|Default|GetPressA) false false)
          (Rendering|SetVisibility (Variables|Default|GethelpDisplay) false false))))
    (:0
      ;[1 1 1] Everything off
      (Rendering|SetVisibility (Variables|Default|GetPressA) false false)
      (Rendering|SetVisibility (Variables|Default|GethelpDisplay) false false)
      (Rendering|SetVisibility (Variables|Default|GetBG) false true))
    (:1
      ;[1 1 1] Press A instructions
      (Rendering|SetVisibility (Variables|Default|GetPressA) true false)
      (Rendering|SetVisibility (Variables|Default|GethelpDisplay) true false)
      (Rendering|SetVisibility (Variables|Default|GetBG) true false))))

(fn ConstructionScript)