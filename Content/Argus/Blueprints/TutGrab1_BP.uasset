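; Grabbable cube for the VR grab tutorial, picked up and dropped through BP_MotionController.
; The first pickup completes the grab step: it plays a beep, turns the cube green, fades it out via a timeline-driven material parameter, then hides it.
; It then starts teleport instructions with timed delays, advancing TutorialStage on TutPointTable_BP and revealing its teleport zone.
; Tick restores the cube at its starting position once the table flags NeedGrab1.
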(event EventBeginPlay
  ;[1 1 1] Set variables at start adn make Grab tut 2 features and 2nd table invisible
  (Variables|Default|SetObjectGrabbed? false)
  (bind _outactors (Actor|GetAllActorsOfClass "/Game/Argus/Blueprints/TutPoint+Table_BP.TutPoint+Table_BP_C"))
  (Variables|Default|SetMainTutREF (Utilities|Array|Get(acopy) _outactors))
  (Variables|Default|SetinitialPosition (Transformation|GetWorldLocation (Variables|Debug|GetStaticMeshComponent))))

(event Collision|EventActorBeginOverlap
  (params (OtherActor :type Actor%20Object%20Reference)))

(event EventTick
  (params (DeltaSeconds :type Float%20%28single-precision%29))
  (bind _staticmeshcomponent (Variables|Debug|GetStaticMeshComponent))
  (if (and (Variables|/Game/Argus/Blueprints/TutPoint+Table_BP.TutPoint+Table_BP_C|GetNeedGrab1? (Variables|Default|GetMainTutREF)) (Math|Boolean|Equal(Boolean) (Variables|Default|GetTutSectionsOn?) false))
    (Variables|Default|SetTutSectionsOn? true)
    (Rendering|SetVisibility _staticmeshcomponent true false)
    (Collision|SetCollisionEnabled _staticmeshcomponent "QueryAndPhysics")
    (Rendering|Material|SetScalarParameterValueonMaterials _staticmeshcomponent "DTAA" 1.0)
    (Rendering|Material|SetVectorParameterValueonMaterials _staticmeshcomponent "BaseColor" "1.000000,1.000000,1.000000")
    (Transformation|SetWorldLocation _staticmeshcomponent (Variables|Default|GetinitialPosition) false false)))

(event EventPickup
  (params (AttachTo :type Scene%20Component%20Object%20Reference))
  (bind _maintutref (Variables|Default|GetMainTutREF))
  (bind _staticmeshcomponent (Variables|Debug|GetStaticMeshComponent))
  (Physics|SetSimulatePhysics (Variables|Debug|GetStaticMeshComponent) false)
  (Transformation|AttachComponentToComponent (VehicleSound|GetRootComponent) AttachTo "eve" "KeepWorld" "KeepWorld" "KeepWorld" false)
  (if (not (Variables|Default|GetObjectGrabbed?)) ; has the grabbing tutorial been completed?
    ;[1 1 1] completing grabbing tutorial
    (Variables|Default|SetObjectGrabbed? true)
    (Audio|PlaySound2D "/Game/Argus/Audio/S_correct_beep_Cue.S_correct_beep_Cue")
    (Rendering|Material|SetVectorParameterValueonMaterials _staticmeshcomponent "DiffuseColor" "0,1.000000, 0")
    (bind _dtaa (Timeline|FadeDTAA Play)
      (:Update
        ;[1 1 1] Make cube fade away until it is needed again
        (Rendering|Material|SetScalarParameterValueonMaterials _staticmeshcomponent "DTAA" _dtaa))
      (:Finished
        (Rendering|SetVisibility _staticmeshcomponent false false)
        (Collision|SetCollisionEnabled _staticmeshcomponent "NoCollision")
        ;[1 1 1] begin teleport instructions
        (Utilities|FlowControl|Delay 1.0)
        (Audio|PlaySound2D "/Game/Argus/Audio/TutD5_S1.TutD5_S1")
        (Variables|/Game/Argus/Blueprints/TutPoint+Table_BP.TutPoint+Table_BP_C|SettutorialStage _maintutref 6)
        (Utilities|FlowControl|Delay 11.0)
        (Variables|/Game/Argus/Blueprints/TutPoint+Table_BP.TutPoint+Table_BP_C|SettutorialStage _maintutref 7)
        (Utilities|FlowControl|Delay 18.0)
        (Rendering|SetVisibility (Variables|/Game/Argus/Blueprints/TutPoint+Table_BP.TutPoint+Table_BP_C|GetTeleportZone _maintutref) true true)
        (Audio|Components|Audio|Play (Variables|/Game/Argus/Blueprints/TutPoint+Table_BP.TutPoint+Table_BP_C|GetTeleportAudio _maintutref) 0.0)))))

(event EventDrop
  (Physics|SetSimulatePhysics (Variables|Debug|GetStaticMeshComponent) true)
  (Transformation|DetachFromActor "KeepWorld" "KeepWorld" "KeepWorld"))

(fn ConstructionScript)