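; VR puzzle dial that the player turns to find the right number and reveal a hidden card.
; While grabbed, the hand's height moves the holder vertically and sets the dial's pitch each tick.
; Nested overlap zones scale right-controller rumble and noise volume toward the target, where a timeline fades the dial green.
; Leaving the target once fully green plays a beep, shows Card1 and disables the dial's collision.
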(event OnComponentEndOverlap(weak1b)
  (params (OverlappedComponent :type Primitive%20Component%20Object%20Reference) (OtherActor :type Actor%20Object%20Reference) (OtherComp :type Primitive%20Component%20Object%20Reference) (OtherBodyIndex :type Integer))
  ;[1 1 1] Vibrate right hand if player in Weak Zone
  (Default|RumbleController (Variables|Default|GetRightControllerREF) 0.6 false)
  (Audio|Components|Audio|Stop (Variables|Default|GetdialNoise)))

(event OnComponentEndOverlap(veryWeak1a)
  (params (OverlappedComponent :type Primitive%20Component%20Object%20Reference) (OtherActor :type Actor%20Object%20Reference) (OtherComp :type Primitive%20Component%20Object%20Reference) (OtherBodyIndex :type Integer))
  ;[1 1 1] Vibrate right hand if player in Weaker Zone
  (Default|RumbleController (Variables|Default|GetRightControllerREF) 0.2 false)
  (Audio|Components|Audio|Stop (Variables|Default|GetdialNoise)))

(event OnComponentBeginOverlap(veryWeak1b)
  (params (OverlappedComponent :type Primitive%20Component%20Object%20Reference) (OtherActor :type Actor%20Object%20Reference) (OtherComp :type Primitive%20Component%20Object%20Reference) (OtherBodyIndex :type Integer) (bFromSweep :type Boolean) (SweepResult :type Hit%20Result%20Structure%20%28by%20ref%29))
  (bind _dialnoise (Variables|Default|GetdialNoise))
  ;[1 1 1] Vibrate right hand if player in Weaker Zone
  (if (and (== OtherComp (Variables|Default|Getdetection)) (Variables|Default|GetDialGrabbed?))
    (Default|RumbleController (Variables|Default|GetRightControllerREF) 0.2 true)
    (Audio|Components|Audio|Play _dialnoise 0.0)
    (Audio|Components|Audio|SetVolumeMultiplier _dialnoise 0.5 :!class /Script/Engine.AudioComponent)))

(event OnComponentEndOverlap(veryWeak1b)
  (params (OverlappedComponent :type Primitive%20Component%20Object%20Reference) (OtherActor :type Actor%20Object%20Reference) (OtherComp :type Primitive%20Component%20Object%20Reference) (OtherBodyIndex :type Integer))
  ;[1 1 1] Vibrate right hand if player in Weaker Zone
  (Default|RumbleController (Variables|Default|GetRightControllerREF) 0.2 false)
  (Audio|Components|Audio|Stop (Variables|Default|GetdialNoise)))

(event OnComponentBeginOverlap(weak1a)
  (params (OverlappedComponent :type Primitive%20Component%20Object%20Reference) (OtherActor :type Actor%20Object%20Reference) (OtherComp :type Primitive%20Component%20Object%20Reference) (OtherBodyIndex :type Integer) (bFromSweep :type Boolean) (SweepResult :type Hit%20Result%20Structure%20%28by%20ref%29))
  (bind _dialnoise (Variables|Default|GetdialNoise))
  ;[1 1 1] Vibrate right hand if player in Weak Zone
  (if (and (== OtherComp (Variables|Default|Getdetection)) (Variables|Default|GetDialGrabbed?))
    (Default|RumbleController (Variables|Default|GetRightControllerREF) 0.6 true)
    (Audio|Components|Audio|Play _dialnoise 0.0)
    (Audio|Components|Audio|SetVolumeMultiplier _dialnoise 1.0 :!class /Script/Engine.AudioComponent)))

(event OnComponentBeginOverlap(weak1b)
  (params (OverlappedComponent :type Primitive%20Component%20Object%20Reference) (OtherActor :type Actor%20Object%20Reference) (OtherComp :type Primitive%20Component%20Object%20Reference) (OtherBodyIndex :type Integer) (bFromSweep :type Boolean) (SweepResult :type Hit%20Result%20Structure%20%28by%20ref%29))
  (bind _dialnoise (Variables|Default|GetdialNoise))
  ;[1 1 1] Vibrate right hand if player in Weak Zone
  (if (and (== OtherComp (Variables|Default|Getdetection)) (Variables|Default|GetDialGrabbed?))
    (Default|RumbleController (Variables|Default|GetRightControllerREF) 0.6 true)
    (Audio|Components|Audio|Play _dialnoise 0.0)
    (Audio|Components|Audio|SetVolumeMultiplier _dialnoise 1.0 :!class /Script/Engine.AudioComponent)))

(event OnComponentEndOverlap(weak1a)
  (params (OverlappedComponent :type Primitive%20Component%20Object%20Reference) (OtherActor :type Actor%20Object%20Reference) (OtherComp :type Primitive%20Component%20Object%20Reference) (OtherBodyIndex :type Integer))
  ;[1 1 1] Vibrate right hand if player in Weak Zone
  (Default|RumbleController (Variables|Default|GetRightControllerREF) 0.6 false)
  (Audio|Components|Audio|Stop (Variables|Default|GetdialNoise)))

(event OnComponentBeginOverlap(strong1)
  (params (OverlappedComponent :type Primitive%20Component%20Object%20Reference) (OtherActor :type Actor%20Object%20Reference) (OtherComp :type Primitive%20Component%20Object%20Reference) (OtherBodyIndex :type Integer) (bFromSweep :type Boolean) (SweepResult :type Hit%20Result%20Structure%20%28by%20ref%29))
  (bind _dialnoise (Variables|Default|GetdialNoise))
  ;[1 1 1] Logic for player contact with the RIGHT number
  (if (== OtherComp (Variables|Default|Getdetection)) ; check that dial detect is overlapping
    (Audio|Components|Audio|Play _dialnoise 0.0)
    (Audio|Components|Audio|SetVolumeMultiplier _dialnoise 1.8 :!class /Script/Engine.AudioComponent)
    (Default|RumbleController (Variables|Default|GetRightControllerREF) 1.0 true) ; loop the rumble
    (bind _fadetogreen (Timeline|ColorChange Play)
      (:Update
        (Rendering|Material|SetVectorParameterValueonMaterials (Variables|Default|GetDial) "DiffuseColor" (Math|Conversions|ToVector(LinearColor) _fadetogreen))
        (Variables|Default|SetRightNumDetected? (Math|Vector|Equal(Vector) (Math|Conversions|ToVector(LinearColor) _fadetogreen) (Variables|Default|GetGreenColor) 0.0001))
        (Variables|Default|SetPlayerWin? true)))))

(event OnComponentEndOverlap(strong1)
  (params (OverlappedComponent :type Primitive%20Component%20Object%20Reference) (OtherActor :type Actor%20Object%20Reference) (OtherComp :type Primitive%20Component%20Object%20Reference) (OtherBodyIndex :type Integer))
  ;[1 1 1] Logic for player contact with the RIGHT number
  (Default|RumbleController (Variables|Default|GetRightControllerREF) 0.0 false) ; stop the rumble loop
  (Audio|Components|Audio|Stop (Variables|Default|GetdialNoise))
  (if (Variables|Default|GetRightNumDetected?) ; check if player held on range 2 long enough
    (Variables|/Script/Engine.PrimitiveComponent|SetbGenerateOverlapEvents (Variables|Default|Getdetection) false) ; Turn off dial detect to stop vibrations
    (Utilities|FlowControl|Delay 1.0)
    (Audio|PlaySound2D "/Game/Argus/Audio/S_correct_beep_Cue.S_correct_beep_Cue") ; play correct sound and sound for card slot
    (Rendering|SetVisibility (Variables|/Script/Engine.StaticMeshActor|GetStaticMeshComponent (Variables|Default|GetCard1_REF)) true false)
    (Collision|SetActorEnableCollision self false)
    (Collision|SetCollisionEnabled (Variables|Default|GetDial) "NoCollision")
    (else
      (bind _fadetogreen (Timeline|ColorChange Reverse)
        (:Update
          (Rendering|Material|SetVectorParameterValueonMaterials (Variables|Default|GetDial) "DiffuseColor" (Math|Conversions|ToVector(LinearColor) _fadetogreen))
          (Variables|Default|SetRightNumDetected? (Math|Vector|Equal(Vector) (Math|Conversions|ToVector(LinearColor) _fadetogreen) (Variables|Default|GetGreenColor) 0.0001))
          (Variables|Default|SetPlayerWin? true))))))

(event OnComponentBeginOverlap(veryWeak1a)
  (params (OverlappedComponent :type Primitive%20Component%20Object%20Reference) (OtherActor :type Actor%20Object%20Reference) (OtherComp :type Primitive%20Component%20Object%20Reference) (OtherBodyIndex :type Integer) (bFromSweep :type Boolean) (SweepResult :type Hit%20Result%20Structure%20%28by%20ref%29))
  (bind _dialnoise (Variables|Default|GetdialNoise))
  ;[1 1 1] Vibrate right hand if player in Weaker Zone
  (if (and (== OtherComp (Variables|Default|Getdetection)) (Variables|Default|GetDialGrabbed?))
    (Default|RumbleController (Variables|Default|GetRightControllerREF) 0.2 true)
    (Audio|Components|Audio|Play _dialnoise 0.0)
    (Audio|Components|Audio|SetVolumeMultiplier _dialnoise 0.5 :!class /Script/Engine.AudioComponent)))

(event EventBeginPlay
  (Variables|Default|SetDialGrabbed? false)
  (bind _outactors (Actor|GetAllActorsOfClass "/Game/VirtualRealityBP/Blueprints/MotionControllerPawn.MotionControllerPawn_C"))
  (Variables|Default|SetRightControllerREF (Variables|/Game/VirtualRealityBP/Blueprints/MotionControllerPawn.MotionControllerPawn_C|GetRightController (Utilities|Array|Get(acopy) _outactors)))
  (Variables|Default|SetHapticIntensity 0.0)
  (Variables|Default|SetRightNumDetected? false)
  (Rendering|Material|CreateDynamicMaterialInstance (Variables|Default|GetDial) 0 "/Game/VirtualReality/Materials/M_BaseMaterial.M_BaseMaterial" :!class /Script/Engine.PrimitiveComponent)
  (Variables|Default|SetDialTutDone? false)
  (Variables|Default|SetHolderInitialPosition (Transformation|GetWorldLocation (Variables|Default|GetHolder)))
  (Variables|Default|SetPlayerWin? false)
  (bind _outactors_2 (Actor|GetAllActorsOfClass "/Game/Argus/Blueprints/Card1_BP.Card1_BP_C"))
  (bind _output_get (Variables|Default|SetCard1_REF (Utilities|Array|Get(acopy) _outactors_2)))
  (Rendering|SetVisibility (Variables|/Script/Engine.StaticMeshActor|GetStaticMeshComponent _output_get) false false)
  (bind _outactors_3 (Actor|GetAllActorsOfClass "/Game/Argus/Blueprints/WallLightPuzzle_BP.WallLightPuzzle_BP_C"))
  (Variables|Default|SetR1WallLightREF (Utilities|Array|Get(acopy) _outactors_3))
  (Audio|Components|Audio|Stop (Variables|Default|GetdialNoise)))

(event Collision|EventActorBeginOverlap
  (params (OtherActor :type Actor%20Object%20Reference)))

(event EventTick
  (params (DeltaSeconds :type Float%20%28single-precision%29))
  (bind _indicator1 (Variables|Default|Getindicator1))
  (if (Variables|Default|GetPlayerWin?)
    (Rendering|Material|SetVectorParameterValueonMaterials _indicator1 "Color1" (Variables|Default|GetGreenColor))
    (Rendering|Material|SetScalarParameterValueonMaterials _indicator1 "Speed" 0.0)
    (else
      (Rendering|Material|SetVectorParameterValueonMaterials (Variables|Default|Getindicator1) "Color1" (Variables|Default|GetYellowColor))))
  (if (Variables|Default|GetDialGrabbed?)
    (CallFunction|DialRotationFeedback)))

(event EventPickup
  (params (AttachTo :type Scene%20Component%20Object%20Reference))
  ;[1 1 1] Dial pickup and let go system
  (if (Collision|IsOverlappingActor (Variables|Default|GetHolder) (Variables|Default|GetRightControllerREF) :!class /Script/Engine.PrimitiveComponent)
    (Variables|Default|SetGrabbingHandREF AttachTo)
    (Variables|Default|SetDialGrabbed? true)))

(event EventDrop
  ;[1 1 1] Dial pickup and let go system
  (Variables|Default|SetDialGrabbed? false)
  (Transformation|SetWorldRotation (Variables|Default|GetDial) "0, 0, 0" false false)
  (Transformation|SetWorldLocation (Variables|Default|GetHolder) (Variables|Default|GetHolderInitialPosition) false false))

(fn ConstructionScript)

(fn RotateDialonGrab
  (bind _grabbinghandref (Variables|Default|GetGrabbingHandREF))
  (bind _holderinitialposition (Variables|Default|GetHolderInitialPosition))
  (bind _returnvalue (Transformation|GetWorldLocation _grabbinghandref))
  (Transformation|SetWorldLocation (Variables|Default|GetHolder) (Math|Vector|MakeVector (.x _holderinitialposition) (.y _holderinitialposition) (.z _returnvalue)) false false)
  (Transformation|SetWorldRotation (Variables|Default|GetDial) (Math|Rotator|MakeRotator 0.0 (* (.z _returnvalue) 5.0) 0.0) false false))

(fn DialRotationFeedback
  (CallFunction|RotateDialonGrab))

(fn GetHapticIntensity
  (bind _detection (Variables|Default|Getdetection))
  (bind _strong1 (Variables|Default|Getstrong1))
  (bind _returnvalue (Transformation|GetWorldLocation _strong1))
  (bind _returnvalue_2 (Transformation|GetWorldLocation _detection))
  (bind _returnvalue_3 (- _returnvalue _returnvalue_2))
  (bind _returnvalue_4 (Math|Vector|VectorLength _returnvalue_3))
  (bind _returnvalue_5 (Math|Float|Round _returnvalue_4))
  (if (Variables|Default|GetPlayerWin?)
    (Variables|Default|SetHapticIntensity 0.0)
    (else
      (Utilities|FlowControl|Sequence
        (:then_0
          (if (and (<= _returnvalue_5 23) (>= _returnvalue_5 11)) ; close from strong collider
            (Variables|Default|SetHapticIntensity 0.4)))
        (:then_1
          (if (and (<= _returnvalue_5 33) (>= _returnvalue_5 24)) ; far from strong collider
            (Variables|Default|SetHapticIntensity 0.2)))
        (:then_2
          (if (<= _returnvalue_5 9) ; Very close
            (Variables|Default|SetHapticIntensity 1.0)))))))