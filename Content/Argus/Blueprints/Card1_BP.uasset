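; Card1_BP is a card actor that a VR motion controller can pick up and drop.
; Pickup disables mesh physics and attaches the root to the given component at socket "eve", while Drop detaches it and enables physics.
; BeginPlay starts the card with physics off and clears a Trigger1Found flag.
; The overlap event is empty, and the nodes that would set that flag and recolor materials are unconnected.
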(event OnComponentBeginOverlap(StaticMeshComponent)
  (params (OverlappedComponent :type Primitive%20Component%20Object%20Reference) (OtherActor :type Actor%20Object%20Reference) (OtherComp :type Primitive%20Component%20Object%20Reference) (OtherBodyIndex :type Integer) (bFromSweep :type Boolean) (SweepResult :type Hit%20Result%20Structure%20%28by%20ref%29)))

(event EventBeginPlay
  (Variables|Default|SetTrigger1Found? false)
  (Physics|SetSimulatePhysics (Variables|Debug|GetStaticMeshComponent) false))

(event Collision|EventActorBeginOverlap
  (params (OtherActor :type Actor%20Object%20Reference)))

(event EventTick
  (params (DeltaSeconds :type Float%20%28single-precision%29)))

(event EventPickup
  (params (AttachTo :type Scene%20Component%20Object%20Reference))
  (Utilities|FlowControl|Sequence
    (:then_0
      (Physics|SetSimulatePhysics (Variables|Debug|GetStaticMeshComponent) false)
      (Transformation|AttachComponentToComponent (VehicleSound|GetRootComponent) AttachTo "eve" "KeepWorld" "KeepWorld" "KeepWorld" false))))

(event EventDrop
  (Physics|SetSimulatePhysics (Variables|Debug|GetStaticMeshComponent) true)
  (Transformation|DetachFromActor "KeepWorld" "KeepWorld" "KeepWorld"))

(fn ConstructionScript)